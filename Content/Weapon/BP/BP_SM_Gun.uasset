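; A grabbable gun actor that the player can pick up, drop and fire.
; Pickup turns off mesh physics, snaps the gun to the given component's "gunSocket" and enables player input, while Drop detaches it, restores physics and disables input.
; While the gun is held, pressing FireLeft spawns a scaled-down BP_A_Projectile at the MuzzleLocation component's position and rotation.
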(event EventPickup
  (params (AttachTo :type Scene%20Component%20Object%20Reference))
  (Utilities|FlowControl|Sequence
    (:then_0
      (Input|EnableInput (Game|GetPlayerController 0)))
    (:then_1
      (Physics|SetSimulatePhysics (Variables|Debug|GetStaticMeshComponent) false)
      (Transformation|AttachComponentToComponent (VehicleSound|GetRootComponent) AttachTo "gunSocket" "SnapToTarget" "SnapToTarget" "KeepWorld" false)
      (Variables|Default|SetisGunInHand? true))))

(event EventDrop
  (Utilities|FlowControl|Sequence
    (:then_0
      (Physics|SetSimulatePhysics (Variables|Debug|GetStaticMeshComponent) true)
      (Transformation|DetachFromActor "KeepWorld" "KeepWorld" "KeepWorld")
      (Variables|Default|SetisGunInHand? false))
    (:then_1
      (Input|DisableInput (Game|GetPlayerController 0)))))

(event Input|ActionEvents|InputActionFireLeft
  (params (Key :type Key%20Structure :default "None"))
  (bind _muzzlelocation (Variables|Default|GetMuzzleLocation))
  (:Pressed
    (if (Variables|Default|GetisGunInHand?)
      (Game|SpawnActorfromClass "/Game/Weapon/BP/BP_A_Projectile.BP_A_Projectile_C" (Math|Transform|MakeTransform (Transformation|GetWorldLocation _muzzlelocation) (Transformation|GetWorldRotation _muzzlelocation) "0.200000,0.200000,0.200000") "Undefined" 0 0))))

(fn ConstructionScript)